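; BP_Mode holds the current interaction mode (VIEW, TALK or GAME) and switches to GAME shortly after BeginPlay.
; Change validates the requested name case-insensitively, stores it, then updates the debug text and selector in layout widgets.
; Each change also shows actors tagged StorageLight outside GAME and moves the player camera to its game position for TALK and GAME, or its initial position for VIEW.
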(event EventBeginPlay
  (Utilities|FlowControl|Delay 0.2)
  (CallFunction|Change "GAME"))

(fn ConstructionScript)

(fn Change
  (params (newMode :type String))
  ;[1 1 1] Validation
  (bind (_isvalid _modename) (CallFunction|Validate newMode))
  (if _isvalid
    ;[1 1 1] Enregistrement
    (Variables|Default|Setmode _modename)
    ;[1 1 1] Debug
    (CallFunction|UpdateWidget)
    (CallFunction|ChangedMode)))

(fn ManageStorageLights
  (bind _outactors (Actor|GetAllActorswithTag "StorageLight"))
  (for _array_element _outactors
    (Rendering|SetVisibility (Variables|/Script/Engine.Actor|GetRootComponent _array_element) (Utilities|Enum|NotEqual(Enum) (Variables|Default|Getmode) "GAME") false)))

(fn ChangeCameraPosition
  (Actor|GetActorOfClass "/Game/Player.Player_C")
  (bind _asplayer (Utilities|Casting|CastToPlayer (Game|GetPlayerCharacter 0)))
  (if (or (Utilities|Enum|Equal(Enum) (Variables|Default|Getmode) "TALK") (Utilities|Enum|Equal(Enum) (Variables|Default|Getmode) "GAME"))
    (Default|MovetoGamePosition _asplayer true)
    (else
      (Default|MovetoInitialPosition _asplayer true))))

(fn ChangedMode
  (CallFunction|ManageStorageLights)
  (CallFunction|ChangeCameraPosition))

(fn Validate
  (params (newMode :type String))
  (bind _returnvalue (Class|KismetStringLibrary|ToUpper newMode))
  (return (Math|Boolean|ORBoolean (Utilities|Enum|Equal(Enum) _returnvalue "VIEW") (Utilities|Enum|Equal(Enum) _returnvalue "TALK") (Utilities|Enum|Equal(Enum) _returnvalue "GAME")) _returnvalue))

(fn UpdateWidget
  (bind _foundwidgets (Widget|GetAllWidgetsOfClass "/Game/WIDGET_Layout.WIDGET_Layout_C" false))
  (for _array_element _foundwidgets
    ;[1 1 1] Debug
    (Variables|/Script/UMG.TextBlock|SetText (Variables|/Game/WIDGET_Layout.WIDGET_Layout_C|Getdebug_mode_content _array_element) (Utilities|Text|ToText(String) (Variables|Default|Getmode)))
    ;[1 1 1] Select
    (Class|ComboBoxString|SetSelectedOption (Variables|/Game/WIDGET_Layout.WIDGET_Layout_C|Getselect_mode _array_element) (Variables|Default|Getmode))))